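; Snake body element Blueprint that gives the first element of a snake its own look and prints location debug output.
; The SetFirstElementType event calls the parent implementation, then swaps the mesh's first material slot to BasicAsset03.
; Tick prints the actor's location every frame, and ActorBeginOverlap prints it in orange as a long-lasting message.
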(event `self.ReceiveTick`
  (params (DeltaSeconds :type "Float (single-precision)"))
  (`KismetSystemLibrary.PrintString` (`KismetStringLibrary.Conv_VectorToString` (`self.K2_GetActorLocation`)) true true (struct :`G` 0.66 :`B` 1.0 :`A` 1.0) DeltaSeconds))

(event `self.ReceiveBeginPlay`)

(event `self.ReceiveActorBeginOverlap`
  (params (OtherActor :type "Actor Object Reference"))
  (`KismetSystemLibrary.PrintString` (`KismetStringLibrary.Conv_VectorToString` (`self.K2_GetActorLocation`)) true true (struct :`R` 1.0 :`G` 0.244746 :`B` 0.084698 :`A` 1.0) 60.0))

(event `self.SetFirstElementType`
  (`parent.SetFirstElementType`)
  (`PrimitiveComponent.SetMaterial` (`self.MeshComponent`) 0 "/Engine/MapTemplates/Materials/BasicAsset03.BasicAsset03"))

(fn `UserConstructionScript`)